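; BP_tyoutin is an enemy Blueprint that provides sideways movement and a player-approach attack behavior.
; Move sweeps the actor along its right vector at Spped scaled by Tick, with IsMoveRight choosing the direction.
; Attack snaps rotation toward the player pawn, then has the AIController move toward it with a wide acceptance radius.
; No caller of either function appears here, and a manual chase calculation is left unconnected.
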(fn `Attack`
  (params (deltaTime :type "Float (double-precision)"))
  (`self.K2_SetActorRotation` (`KismetMathLibrary.FindLookAtRotation` (`self.K2_GetActorLocation`) (`self.K2_GetActorLocation` (`GameplayStatics.GetPlayerPawn` 0))))
  (`AIController.MoveToActor` (cast `AIController` (`self.GetController`) :!pure true) (`GameplayStatics.GetPlayerPawn` 0) 500.0 true true true null true))

(fn `Move`
  (params (tick :type "Float (double-precision)"))
  (bind _returnvalue (`self.K2_GetActorLocation`))
  (bind _returnvalue_2 (* (`self.GetActorRightVector`) (* tick (`self.Spped`))))
  (if (`self.IsMoveRight`)
    (`self.K2_SetActorLocation` (+ _returnvalue _returnvalue_2) true)
    (else
      (`self.K2_SetActorLocation` (+ _returnvalue (* _returnvalue_2 -1)) true)))
  (return))

(fn `UserConstructionScript`
  (`parent.UserConstructionScript`))